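; Player controller that creates the lobby UI and relays text chat between players.
; ClientPostLogin builds the LobbyMain widget for the local controller, shows the cursor and switches to UI-only input.
; GetChatMessage reads the controller list from BP_GameMode and calls UpdateChat on each, with an empty sender name.
; UpdateChat forwards the text to the lobby's chat window on the owning client.
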(event Custom|GetChatMessage
  (params (TextToSend :type Text))
  ;[1 1 1] Process incoming chat message and tells all player controllers to run Update Chat
  (Variables|Default|SetSenderText TextToSend)
  (bind _asbp_game_mode (Utilities|Casting|CastToBP_GameMode (Game|GetGameMode)))
  (for _array_element (Variables|/Game/shiratori/Blueprints/BP_GameMode.BP_GameMode_C|GetAllPlayerControllers _asbp_game_mode)
    (CallFunction|UpdateChat _array_element "" (Variables|Default|GetSenderText))))

(event Custom|UpdateChat
  (params (Sender :type Text) (Text :type Text))
  ;[1 1 1] Updates the Chat Display on Owing Client
  (Default|UpdateChatWindow (Variables|/Game/shiratori/Widgets/LobbyMain.LobbyMain_C|GetChatWindow (Variables|Default|GetLobbyMain)) Sender Text))

(event Custom|ClientPostLogin
  (CallFunction|SetupIngameUI))

(event EventBeginPlay)

(event EventTick
  (params (DeltaSeconds :type Float%20%28single-precision%29)))

(fn ConstructionScript)

(fn SetupIngameUI
  (bind _self self)
  (if (Pawn|IsLocalPlayerController)
    (bind _returnvalue (UserInterface|CreateWidget "/Game/shiratori/Widgets/LobbyMain.LobbyMain_C" _self))
    (bind _output_get (Variables|Default|SetLobbyMain _returnvalue))
    (UserInterface|Viewport|AddtoViewport _output_get 0)
    (Variables|Default|SetbShowMouseCursor _self true)
    (Input|SetInputModeUIOnly _self _output_get "DoNotLock")))